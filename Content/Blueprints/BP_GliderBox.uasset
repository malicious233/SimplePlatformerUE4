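; BP_GliderBox is a player-steered box with simple glider-style controls.
; Each tick, vertical and horizontal input add pitch and yaw to Body, scaled by per-axis speeds and delta time.
; Body's rotation is then rebuilt from its forward vector through a quaternion, which discards roll.
; Pressing Jump applies a single unscaled force along that forward vector, with no other flight physics in the graph.
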(event `self.ReceiveTick`
  (params (DeltaSeconds :type "Float (single-precision)"))
  (bind _body (`self.Body`))
  (`SceneComponent.K2_AddRelativeRotation` _body (`KismetMathLibrary.MakeRotator` 0.0 (* (`self.GetInputAxisValue`) (`self.PitchRotSpeed`) DeltaSeconds) (* DeltaSeconds (`self.GetInputAxisValue`) (`self.YawRotSpeed`))) false false)
  (`SceneComponent.K2_SetWorldRotation` _body (`KismetMathLibrary.Quat_Rotator` (`KismetMathLibrary.Conv_VectorToQuaternion` (`SceneComponent.GetForwardVector` _body))) false false))

(event `InputAction|Jump`
  (params (Key :type "Key Structure"))
  (bind _body (`self.Body`))
  (:`Pressed`
    (`PrimitiveComponent.AddForce` _body (`SceneComponent.GetForwardVector` _body) "None" false)))

(fn `UserConstructionScript`)