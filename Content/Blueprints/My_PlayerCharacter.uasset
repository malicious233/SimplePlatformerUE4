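; Player character Blueprint for a physics-driven, camera-relative controller with mouse look, jumping, a forward impulse dash and an attack.
; Each Tick, PFCharFloater hovers the body and sets Grounded, then PFCharMovement applies acceleration and friction.
; Sliding (crouch held), ground and airborne data assets supply the tuning for each state.
; Jump briefly disables the float before applying force, and Attack1 passes FlurryAttack1 to CCAttacker.
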(event `self.ReceiveTick`
  (params (DeltaSeconds :type "Float (single-precision)"))
  (bind _camera (`self.Camera`))
  (bind _pfcharfloater (`self.PFCharFloater`))
  (bind _pfcharmovement (`self.PFCharMovement`))
  (bind _groundmovementdataasset (`self.GroundMovementDataAsset`))
  (bind _groundmovementdataasset_2 (`self.GroundMovementDataAsset`))
  (bind _slidingmovementdataasset (`self.SlidingMovementDataAsset`))
  (bind _airbornemovementdataasset (`self.AirborneMovementDataAsset`))
  (bind _slidingmovementdataasset_2 (`self.SlidingMovementDataAsset`))
  (bind _pfcharmovement_2 (`self.PFCharMovement`))
  (bind _returnvalue (`KismetMathLibrary.Normal` (`KismetMathLibrary.MakeVector` (.x (+ (* (`KismetMathLibrary.Conv_DoubleToVector` (`self.GetInputAxisValue`)) (`SceneComponent.GetForwardVector` _camera)) (* (`SceneComponent.GetRightVector` _camera) (`KismetMathLibrary.Conv_DoubleToVector` (`self.GetInputAxisValue`))))) (.y (+ (* (`KismetMathLibrary.Conv_DoubleToVector` (`self.GetInputAxisValue`)) (`SceneComponent.GetForwardVector` _camera)) (* (`SceneComponent.GetRightVector` _camera) (`KismetMathLibrary.Conv_DoubleToVector` (`self.GetInputAxisValue`))))))))
  (if (`self.Crouching`)
    (bind _returnvalue_2 (`PFCharFloater.Hover` _pfcharfloater (`CharacterMovementDataAsset.HoverRay` _slidingmovementdataasset_2) (`CharacterMovementDataAsset.HoverDistance` _slidingmovementdataasset_2) (`CharacterMovementDataAsset.HoverStrength` _slidingmovementdataasset_2) (`CharacterMovementDataAsset.HoverDamping` _slidingmovementdataasset_2)))
    (set `self.Grounded` _returnvalue_2)
    (else
      (bind _returnvalue_3 (`PFCharFloater.Hover` _pfcharfloater (`CharacterMovementDataAsset.HoverRay` _groundmovementdataasset) (`CharacterMovementDataAsset.HoverDistance` _groundmovementdataasset) (`CharacterMovementDataAsset.HoverStrength` _groundmovementdataasset) (`CharacterMovementDataAsset.HoverDamping` _groundmovementdataasset)))
      (bind _output_get (set `self.Grounded` _returnvalue_3))))
  (if _output_get
    (if (`self.Crouching`)
      (`PFCharMovement.Move` _pfcharmovement _returnvalue (`CharacterMovementDataAsset.Acceleration` _slidingmovementdataasset) (`CharacterMovementDataAsset.MaxSpeed` _slidingmovementdataasset))
      (`PFCharMovement.ApplyFriction` _pfcharmovement_2 (`CharacterMovementDataAsset.Deacceleration` (`self.SlidingMovementDataAsset`)))
      (else
        (`PFCharMovement.Move` _pfcharmovement _returnvalue (`CharacterMovementDataAsset.Acceleration` _groundmovementdataasset_2) (`CharacterMovementDataAsset.MaxSpeed` _groundmovementdataasset_2))
        (`PFCharMovement.ApplyFriction` _pfcharmovement_2 (`CharacterMovementDataAsset.Deacceleration` (`self.GroundMovementDataAsset`)))))
    (else
      (`PFCharMovement.Move` _pfcharmovement _returnvalue (`CharacterMovementDataAsset.Acceleration` _airbornemovementdataasset) (`CharacterMovementDataAsset.MaxSpeed` _airbornemovementdataasset))
      (`PFCharMovement.ApplyFriction` _pfcharmovement_2 (`CharacterMovementDataAsset.Deacceleration` (`self.AirborneMovementDataAsset`))))))

(event `InputAction|Dash`
  (params (Key :type "Key Structure"))
  (:`Pressed`
    (`PrimitiveComponent.AddImpulse` (`self.Collider`) (* (`SceneComponent.GetForwardVector` (`self.Camera`)) 1500.0) "None" true)))

(event `InputAction|Jump`
  (params (Key :type "Key Structure"))
  (:`Pressed`
    (if (`self.Grounded`)
      (`PFCharFloater.BrieflyDisableFloat` (`self.PFCharFloater`))
      (`PFCharMovement.Jump` (`self.PFCharMovement`) (`self.JumpForce`)))))

(event `InputAxis|MouseY`
  (params (AxisValue :type "Float (single-precision)"))
  (`self.AddControllerPitchInput` (* AxisValue (`self.MouseSensitivity`))))

(event `InputAxis|Crouch`
  (params (AxisValue :type "Float (single-precision)"))
  (bind _output_get (set `self.Crouching` (>= AxisValue 1.0)))
  (`KismetSystemLibrary.PrintString` (`KismetStringLibrary.Conv_BoolToString` _output_get) true true (struct :`G` 0.66 :`B` 1.0 :`A` 1.0) 0.0))

(event `InputAxis|MouseX`
  (params (AxisValue :type "Float (single-precision)"))
  (`self.AddControllerYawInput` (* (`self.MouseSensitivity`) AxisValue)))

(event `InputAction|Attack1`
  (params (Key :type "Key Structure"))
  (:`Pressed`
    (`CCAttacker.PerformAttack` (`self.CCAttacker`) (`self.FlurryAttack1`))))

(fn `UserConstructionScript`)