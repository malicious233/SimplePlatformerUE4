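; FlurryAttack is an attack Blueprint that fires two timed hits in sequence, currently only as debug prints with no damage logic.
; OnAttackStart resets two boolean latches, and OnAttackTick checks each against its own time threshold.
; A reusable TimingCondition helper compares TimeSinceAttackStart to the threshold and sets the latch by reference, so each hit fires once per attack.
; NewFunction_0 is an empty stub.
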(event `self.OnAttackStart`
  (`KismetSystemLibrary.PrintString` "Start FlurryAttack")
  (set `self.Condition1` false)
  (set `self.Condition2` false))

(event `self.OnAttackTick`
  (params (DeltaTime :type "Float (single-precision)"))
  (`self.TimingCondition` (`self.Condition1`)
    (:`True`
      (`KismetSystemLibrary.PrintString` "Smack1" true true (struct :`G` 0.66 :`B` 1.0 :`A` 1.0) 1.0))
    (:`False`
      _))
  (`self.TimingCondition` (`self.Condition2`) 0.75
    (:`True`
      (`KismetSystemLibrary.PrintString` "Smack2" true true (struct :`G` 0.66 :`B` 1.0 :`A` 1.0) 1.0))))

(fn `NewFunction_0`
  (params (NewParam :type Boolean)))